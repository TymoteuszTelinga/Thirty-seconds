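; BP_PlayerControler is a player controller that manages the game's main UI screens.
; It adds the HUD widget on BeginPlay.
; GameHasEnded shows a win or lose screen based on PlayerWin, and ShowShop opens the shop widget.
; Both events clear existing widgets, switch to UI-only input, disable pawn input and show the mouse cursor.
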(event `self.ReceiveBeginPlay`
  (bind _returnvalue (`|CreateWidget` "/Game/BluePrints/Widgets/WBP_HUD.WBP_HUD_C" self))
  (`UserWidget.AddToViewport` _returnvalue 0))

(event `GameHasEnded`
  (params (bPlayerWin :type Boolean))
  (`WidgetLayoutLibrary.RemoveAllWidgets`)
  (bind _returnvalue (`|CreateWidget` (select `bool` bPlayerWin :`false` "/Game/BluePrints/Widgets/WBP_LoseScreen.WBP_LoseScreen_C" :`true` "/Game/BluePrints/Widgets/WBP_WinScreen.WBP_WinScreen_C" :!type "UserWidget Class Reference") self))
  (`WidgetBlueprintLibrary.SetInputMode_UIOnlyEx` self _returnvalue)
  (`UserWidget.AddToViewport` _returnvalue 0)
  (`self.DisableInput` (`self.K2_GetPawn` self) self)
  (set `self.bShowMouseCursor` true))

(event `ShowShop`
  (`WidgetLayoutLibrary.RemoveAllWidgets`)
  (bind _returnvalue (`|CreateWidget` "/Game/BluePrints/Widgets/WBP_Shop.WBP_Shop_C"))
  (`WidgetBlueprintLibrary.SetInputMode_UIOnlyEx` self _returnvalue)
  (`UserWidget.AddToViewport` _returnvalue 0)
  (`self.DisableInput` (`self.K2_GetPawn`) null)
  (set `self.bShowMouseCursor` true))

(fn `UserConstructionScript`)
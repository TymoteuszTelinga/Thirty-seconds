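; Game mode for a shard-collecting level: tracks the quota, activates the gate when it is met, handles deaths and advances levels via LevelInfo_DT.
; Delay-throttled Tick runs a countdown that changes floor tiles and collapses the gate at zero.
; Shard pickups add time, which rewinds tiles.
; Tiles still valid serve as random spawn points for shards and enemies, with normal/spear mix and spawn threshold taken from the level row.
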(event `self.ReceiveBeginPlay`
  (bind _outactors (`GameplayStatics.GetAllActorsOfClass` "/Game/BluePrints/BP_FlorTile.BP_FlorTile_C"))
  (bind _output_get (set `self.FlorTiles` _outactors))
  (set `self.ValidFlor` _output_get)
  (`self.Spawn Shard`)
  (set `self.GameInstRef` (cast `/Game/BluePrints/BP_GameInstance` (`GameplayStatics.GetGameInstance`) :!pure true))
  (set `self.shardToColect` (`/Game/BluePrints/BP_GameInstance.ShardsToColect` (`self.GameInstRef`)))
  (bind _returnvalue (`|GetDataTableRow` "/Game/BluePrints/LevelInfo_DT.LevelInfo_DT" (`/Game/BluePrints/BP_GameInstance.CurentLevel` (`self.GameInstRef`)))
    (:`then`
      (bind _output_get_2 (set `self.LevelInfo` _returnvalue))
      (`KismetSystemLibrary.PrintString` (`KismetStringLibrary.Conv_IntToString` (break `/Game/BluePrints/LevelInfo` _output_get_2))))))

(event `self.ReceiveTick`
  (params (DeltaSeconds :type "Float (single-precision)"))
  (`|ExecutionSequence`
    (:`then_0`
      (`KismetSystemLibrary.Delay` 2.0)
      (if (not (`self.bGameEnded`))
        (`self.Spawn Enemys`)))
    (:`then_1`
      (`KismetSystemLibrary.Delay` 1.0)
      (if (`self.bAddTime`)
        (bind _output_get (set `self.Seconds` (`KismetMathLibrary.Clamp` (+ 1 (`self.Seconds`)) 0 30)))
        (if (>= _output_get 30)
          (set `self.bAddTime` false)
          (else
            (bind _result (`/Engine/EditorBlueprintResources/StandardMacros.DecrementInt` (`self.seconds to add`))
              (:`  `
                (set `self.bAddTime` (> _result 0))))))
        (for _array_element (`self.FlorTiles`)
          (`/Game/BluePrints/BP_FlorTile.RewindTime` _array_element)
          (`KismetArrayLibrary.Array_Clear` (`self.ValidFlor`) :!label _label)
          (for _array_element_2 (`self.FlorTiles`)
            (if (`/Game/BluePrints/BP_FlorTile.IsFlorValid` _array_element_2)
              (`KismetArrayLibrary.Array_Add` (`self.ValidFlor`) _array_element_2))))
        (else
          (bind _result_2 (`/Engine/EditorBlueprintResources/StandardMacros.DecrementInt` (`self.Seconds`))
            (:`  `
              (if (<= _result_2 0)
                (bind _returnvalue (`GameplayStatics.GetActorOfClass` "/Game/BluePrints/BP_Gate.BP_Gate_C"))
                (`/Engine/EditorBlueprintResources/StandardMacros.IsValid` _returnvalue
                  (:`Is Valid`
                    (`/Game/BluePrints/BP_Gate.Colaps` _returnvalue))
                  (:`Is Not Valid`
                    _)))
              (for _array_element_3 (`self.FlorTiles`)
                (`/Game/BluePrints/BP_FlorTile.TimeChange` _array_element_3 (`self.Seconds`))
                (goto _label)))))))))

(event `AddTime`
  (params (Seconds :type Integer))
  (set `self.seconds to add` Seconds)
  (set `self.bAddTime` true))

(event `SharpCollect`
  (bind _result (`/Engine/EditorBlueprintResources/StandardMacros.IncrementInt` (`self.ColectedShards`))
    (:`  `
      (if (>= _result (`self.shardToColect`))
        (`self.AddTime` 3)
        (bind _returnvalue (`GameplayStatics.GetActorOfClass` "/Game/BluePrints/BP_Gate.BP_Gate_C"))
        (`/Game/BluePrints/BP_Gate.ActiveGate` _returnvalue)
        (set `self.bGameEnded` true)
        (bind _outactors (`GameplayStatics.GetAllActorsOfClass` "/Game/BluePrints/Enemy/BP_Enemy.BP_Enemy_C"))
        (for _array_element _outactors
          (`self.K2_DestroyActor` _array_element))
        (`self.SetActorTickEnabled` false)
        (for _array_element_2 (`self.FlorTiles`)
          (`/Game/BluePrints/BP_FlorTile.RewindTime` _array_element_2))
        (else
          (`self.AddTime` 3)
          (`self.Spawn Shard`))))))

(event `Actor died`
  (params (DeadActor :type "Actor Object Reference"))
  (bind _asbp_enemy (cast `/Game/BluePrints/Enemy/BP_Enemy` DeadActor)
    (:`then`
      (`self.K2_DestroyActor` _asbp_enemy)
      (`/Engine/EditorBlueprintResources/StandardMacros.DecrementInt` (`self.EnemyInLevel`)))
    (:`CastFailed`
      (bind _asbp_character (cast `/Game/BluePrints/BP_CHaracter` DeadActor)
        (:`then`
          (bind _asbp_player_controler (cast `/Game/BluePrints/BP_PlayerControler` (`Pawn.GetController` _asbp_character)))
          (`/Game/BluePrints/BP_PlayerControler.GameHasEnded` _asbp_player_controler false)
          (set `self.bGameEnded` true)
          (`self.K2_DestroyActor` _asbp_character))
        (:`CastFailed`
          (`self.K2_DestroyActor` DeadActor))))))

(event `NextLewel`
  (bind (_spearenemy _normalenemy _nextlevel) (break `/Game/BluePrints/LevelInfo` (`self.LevelInfo`)))
  (if (== _nextlevel "None")
    (bind _asbp_player_controler (cast `/Game/BluePrints/BP_PlayerControler` (`GameplayStatics.GetPlayerController` 0)))
    (`/Game/BluePrints/BP_PlayerControler.GameHasEnded` _asbp_player_controler true)
    (else
      (bind _output_get (set `/Game/BluePrints/BP_GameInstance.CurentLevel` _nextlevel (`self.GameInstRef`)))
      (`GameplayStatics.OpenLevel` _output_get))))

(fn `Spawn Enemys`
  (bind _validflor (`self.ValidFlor`))
  (bind (_levelinfo_spearenemy _levelinfo_normalenemy) (break `/Game/BluePrints/LevelInfo` (`self.LevelInfo`)))
  (bind (_levelinfo_spearenemy_2 _levelinfo_normalenemy_2) (break `/Game/BluePrints/LevelInfo` (`self.LevelInfo`)))
  (bind _returnvalue (+ (`self.K2_GetActorLocation` (`|GetArrayItem` _validflor (`KismetMathLibrary.RandomInteger` (`KismetArrayLibrary.Array_Length` _validflor)))) (0.0 0.0 80.0)))
  (if (< (`self.EnemyInLevel`) (+ _levelinfo_spearenemy _levelinfo_normalenemy))
    (if (> (`KismetArrayLibrary.Array_Length` (`self.ValidFlor`)) 0)
      (for _ (range 1 (+ (`KismetMathLibrary.RandomIntegerInRange` 2 4) 1))
        (if (`KismetMathLibrary.RandomBoolWithWeight` (- 1.0 (/ (`KismetMathLibrary.Conv_IntToDouble` _levelinfo_spearenemy_2) (`KismetMathLibrary.Conv_IntToDouble` (+ _levelinfo_spearenemy_2 _levelinfo_normalenemy_2)))))
          (bind _returnvalue_2 (`AIBlueprintHelperLibrary.SpawnAIFromClass` "/Game/BluePrints/Enemy/BP_Enemy.BP_Enemy_C" "/Game/BluePrints/Enemy/BT_Enemy.BT_Enemy" _returnvalue (struct) false null))
          (`/Engine/EditorBlueprintResources/StandardMacros.IsValid` _returnvalue_2
            (:`Is Valid`
              (`/Engine/EditorBlueprintResources/StandardMacros.IncrementInt` (`self.EnemyInLevel`))))
          (else
            (bind _returnvalue_3 (`AIBlueprintHelperLibrary.SpawnAIFromClass` "/Game/BluePrints/Enemy/BP_Enemy_Spear.BP_Enemy_Spear_C" "/Game/BluePrints/Enemy/BT_Enemy_Spear.BT_Enemy_Spear" _returnvalue (struct) false null))
            (`/Engine/EditorBlueprintResources/StandardMacros.IsValid` _returnvalue_3
              (:`Is Valid`
                (`/Engine/EditorBlueprintResources/StandardMacros.IncrementInt` (`self.EnemyInLevel`))))))))))

(fn `Spawn Shard`
  (bind _validflor (`self.ValidFlor`))
  (if (`KismetArrayLibrary.Array_IsValidIndex` (`self.ValidFlor`))
    (bind _returnvalue (`|SpawnActorFromClass` "/Game/BluePrints/BP_shard.BP_shard_C" (`KismetMathLibrary.Conv_VectorToTransform` (+ (`self.K2_GetActorLocation` (`|GetArrayItem` _validflor (`KismetMathLibrary.RandomInteger` (`KismetArrayLibrary.Array_Length` _validflor)))) (0.0 0.0 80.0))) "DontSpawnIfColliding" "OverrideRootScale" null null :!label _label))
    (`/Engine/EditorBlueprintResources/StandardMacros.IsValid` _returnvalue
      (:`Is Not Valid`
        (goto _label)))))

(fn `UserConstructionScript`)
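; BP_shard is a collectible shard pickup that reports to the main game mode when the player character collects it.
; On BeginPlay, the UpAndDown timeline lifts the shard component from its starting relative location and adds a fixed local rotation each update, so the spin depends on frame rate.
; A capsule overlap with BP_Character calls SharpCollect on BP_MainGameMode, then destroys the actor.
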(event `self.ReceiveBeginPlay`
  (bind _shard (`self.Shard`))
  (set `self.Base Location` (`SceneComponent.RelativeLocation` (`self.Shard`)))
  (bind (_direction _alpha) (`Timeline|UpAndDown`)
    (:`Update`
      (`SceneComponent.K2_SetRelativeLocation` _shard (+ (`self.Base Location`) (`KismetMathLibrary.MakeVector` 0.0 0.0 (`KismetMathLibrary.Lerp` 0.0 30.0 _alpha))) false false)
      (`SceneComponent.K2_AddLocalRotation` _shard (struct :`Yaw` 1.0) false false))))

(event `self.ReceiveTick`
  (params (DeltaSeconds :type "Float (single-precision)")))

(event `self.Capsule.OnComponentBeginOverlap`
  (params (OverlappedComponent :type "PrimitiveComponent Object Reference") (OtherActor :type "Actor Object Reference") (OtherComp :type "PrimitiveComponent Object Reference") (OtherBodyIndex :type Integer) (bFromSweep :type Boolean) (SweepResult :type "HitResult Structure (by ref)"))
  (cast `/Game/BluePrints/BP_CHaracter` OtherActor)
  (bind _asbp_main_game_mode (cast `/Game/BluePrints/BP_MainGameMode` (`GameplayStatics.GetGameMode`)))
  (`/Game/BluePrints/BP_MainGameMode.SharpCollect` _asbp_main_game_mode)
  (`self.K2_DestroyActor`))

(fn `UserConstructionScript`)
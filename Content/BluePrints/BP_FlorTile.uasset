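; BP_FlorTile is a floor tile that collapses at a random point in time and can rewind to where it was.
; TimeChange starts physics once Seconds drops below the random ColapsTime picked at BeginPlay, otherwise stops falling, as does RewindTime.
; While falling, Tick records transform and velocities into RewindPath; otherwise it disables physics and pops one state per frame.
; IsFlorValid reports when that path is nearly or fully empty.
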(event `self.ReceiveBeginPlay`
  ;[1 1 1] Colaps Time
  (set `self.ColapsTime` (`KismetMathLibrary.RandomIntegerInRange` 0 30)))

(event `TimeChange`
  (params (Seconds :type Integer))
  (if (< Seconds (`self.ColapsTime`))
    (`PrimitiveComponent.SetSimulatePhysics` (`self.Cube`) true)
    (set `self.bFalling` true)
    (else
      (set `self.bFalling` false :!label _label))))

(event `RewindTime`
  (goto _label))

(event `self.ReceiveTick`
  (params (DeltaSeconds :type "Float (single-precision)"))
  (bind _rewindpath (`self.RewindPath`))
  (bind _returnvalue (`KismetArrayLibrary.Array_LastIndex` _rewindpath))
  (if (`self.bFalling`)
    ;[1 1 1] SetRewindPath
    (`KismetArrayLibrary.Array_Add` (`self.RewindPath`) (`self.GetTileState`))
    (else
      (`PrimitiveComponent.SetSimulatePhysics` (`self.Cube`) false)
      ;[1 1 1] Rewind
      (if (>= _returnvalue 0)
        (`self.SetTileState` (`|GetArrayItem` _rewindpath _returnvalue))
        (`KismetArrayLibrary.Array_Remove` _rewindpath (`KismetArrayLibrary.Array_LastIndex` _rewindpath))))))

(fn `GetTileState`
  (returns (TileState :type "/Game/BluePrints/TileState Structure"))
  (bind _cube (`self.Cube`))
  (bind _returnvalue (`PrimitiveComponent.GetPhysicsLinearVelocity` _cube "None"))
  (return (make `/Game/BluePrints/TileState` (`SceneComponent.K2_GetComponentToWorld` _cube) _returnvalue (`PrimitiveComponent.GetPhysicsAngularVelocityInDegrees` _cube "None"))))

(fn `IsFlorValid`
  (returns (IsValid :type Boolean))
  (return (<= (`KismetArrayLibrary.Array_LastIndex` (`self.RewindPath`)) 0)))

(fn `SetTileState`
  (params (TileState :type "/Game/BluePrints/TileState Structure"))
  (bind (_transform _linearvelocity _angularvelocity) (break `/Game/BluePrints/TileState` TileState))
  (bind _cube (`self.Cube`))
  (`SceneComponent.K2_SetWorldTransform` _cube _transform false false)
  (`PrimitiveComponent.SetPhysicsLinearVelocity` _cube _linearvelocity false "None")
  (`PrimitiveComponent.SetPhysicsAngularVelocityInDegrees` _cube _angularvelocity false "None"))

(fn `UserConstructionScript`
  (`PrimitiveComponent.SetMaterial` (`self.Cube`) 0 (`self.Material`)))
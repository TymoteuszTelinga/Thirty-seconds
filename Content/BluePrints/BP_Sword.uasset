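; BP_Sword is a spinning sword actor that damages enemies it overlaps and reports back to the owning character when destroyed.
; Each BP_Enemy hit applies damage and decrements a pierce counter, destroying the sword when the count runs out, while any other overlap destroys it immediately.
; Destruction calls ReturnSword on the owning BP_Character, and Tick spins the static mesh by a fixed per-frame step, independent of delta time.
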(event `self.ReceiveBeginPlay`)

(event `self.ReceiveActorBeginOverlap`
  (params (OtherActor :type "Actor Object Reference"))
  (bind _asbp_enemy (cast `/Game/BluePrints/Enemy/BP_Enemy` OtherActor)
    (:`then`
      (`GameplayStatics.ApplyDamage` _asbp_enemy 100.0 (`self.GetInstigatorController`) self)
      (bind _result (`/Engine/EditorBlueprintResources/StandardMacros.DecrementInt` (`self.numberOfPierce`))
        (:`  `
          (if (not (> _result 0))
            (`self.K2_DestroyActor`)))))
    (:`CastFailed`
      (`self.K2_DestroyActor`))))

(event `self.ReceiveDestroyed`
  (bind _returnvalue (`self.GetOwner`))
  (`/Engine/EditorBlueprintResources/StandardMacros.IsValid` _returnvalue
    (:`Is Valid`
      (bind _asbp_character (cast `/Game/BluePrints/BP_CHaracter` _returnvalue))
      (`/Game/BluePrints/BP_CHaracter.Return Sword` _asbp_character))))

(event `self.ReceiveTick`
  (params (DeltaSeconds :type "Float (single-precision)"))
  (`SceneComponent.K2_AddLocalRotation` (`self.StaticMesh`) (struct :`Yaw` 1.0) false false))

(fn `UserConstructionScript`)
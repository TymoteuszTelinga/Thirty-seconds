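; BP_Enemy is an enemy actor that damages the player character on overlap and can leave a coin behind.
; On spawn it plays an effect and briefly ignores Pawn collision before restoring blocking.
; Any damage it takes, regardless of amount, is reported to BP_MainGameMode as its death via ActorDied.
; When destroyed it plays a death effect and randomly spawns a BP_Coin at its location.
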(event `self.ReceiveBeginPlay`
  (bind _capsulecomponent (`self.CapsuleComponent`))
  (`GameplayStatics.SpawnEmitterAtLocation` "/Game/Effects/P_SpawnEffect.P_SpawnEffect" (`self.K2_GetActorLocation`))
  (`PrimitiveComponent.SetCollisionResponseToChannel` _capsulecomponent "ECC_Pawn" "ECR_Ignore")
  (`KismetSystemLibrary.Delay` 0.5)
  (`PrimitiveComponent.SetCollisionResponseToChannel` _capsulecomponent "ECC_Pawn" "ECR_Block"))

(event `self.ReceiveDestroyed`
  ;[1 1 1] after death
  (`GameplayStatics.SpawnEmitterAtLocation` "/Game/Effects/P_DeathEffect.P_DeathEffect" (`self.K2_GetActorLocation`))
  (if (> (`KismetMathLibrary.RandomFloat`) 0.5)
    (`|SpawnActorFromClass` "/Game/BluePrints/BP_Coin.BP_Coin_C" (`KismetMathLibrary.MakeTransform` (`self.K2_GetActorLocation`) (struct) (2.0 2.0 2.0)) "Undefined" "OverrideRootScale" null null)))

(event `self.ReceiveAnyDamage`
  (params (Damage :type "Float (single-precision)") (DamageType :type "DamageType Object Reference") (InstigatedBy :type "Controller Object Reference") (DamageCauser :type "Actor Object Reference"))
  ;[1 1 1] TakeDamage
  (bind _asbp_main_game_mode (cast `/Game/BluePrints/BP_MainGameMode` (`GameplayStatics.GetGameMode`)))
  (`/Game/BluePrints/BP_MainGameMode.Actor died` _asbp_main_game_mode self))

(event `self.ReceiveActorBeginOverlap`
  (params (OtherActor :type "Actor Object Reference"))
  ;[1 1 1] Attak Player
  (bind _asbp_character (cast `/Game/BluePrints/BP_CHaracter` OtherActor))
  (`GameplayStatics.ApplyDamage` _asbp_character 100.0))

(fn `UserConstructionScript`)
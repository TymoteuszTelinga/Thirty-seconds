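; Spear-wielding enemy Blueprint that extends a parent class with a weapon attachment and spawn collision handling.
; The construction script sets HasSpear and snaps a skeletal mesh component to the hand socket of the character mesh.
; After parent BeginPlay, the capsule ignores the Pawn channel for half a second, then switches to overlapping it.
; A helper function, IncreseSpeed, sets the character's max walk speed.
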(event `self.ReceiveBeginPlay`
  (bind _capsule (`self.Capsule`))
  (`|ExecutionSequence`
    (:`then_0`
      (`parent.ReceiveBeginPlay`))
    (:`then_1`
      (`PrimitiveComponent.SetCollisionResponseToChannel` _capsule "ECC_Pawn" "ECR_Ignore")
      (`KismetSystemLibrary.Delay` 0.5)
      (`PrimitiveComponent.SetCollisionResponseToChannel` _capsule "ECC_Pawn" "ECR_Overlap"))))

(fn `IncreseSpeed`
  (params (NewSpeed :type "Float (double-precision)" :default 400.0))
  (set `CharacterMovementComponent.MaxWalkSpeed` NewSpeed (`self.CharacterMovement`)))

(fn `UserConstructionScript`
  (`parent.UserConstructionScript`)
  (set `self.bHasSpear` true)
  (`SceneComponent.K2_AttachToComponent` (`self.SkeletalMesh`) (`self.Mesh`) "HandSocet" "SnapToTarget" "SnapToTarget" "KeepRelative" true))
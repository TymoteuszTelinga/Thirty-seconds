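; Behavior tree service for enemy AI that updates a blackboard key with the player pawn when the enemy detects them.
; Each tick it checks that player pawn 0 is valid, visible through the AI controller's line of sight, and within DetectRadius of the owner.
; If any check fails, it clears the key.
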(event `self.ReceiveTick`
  (params (OwnerActor :type "Actor Object Reference") (DeltaSeconds :type "Float (single-precision)"))
  (bind _returnvalue (`GameplayStatics.GetPlayerPawn` 0))
  (bind _key (`self.Key`))
  (`/Engine/EditorBlueprintResources/StandardMacros.IsValid` _returnvalue
    (:`Is Valid`
      (if (and (`Controller.LineOfSightTo` (`AIBlueprintHelperLibrary.GetAIController` OwnerActor) _returnvalue (0.0 0.0 0.0) false) (< (`KismetMathLibrary.VSize` (- (`Actor.K2_GetActorLocation` OwnerActor) (`Actor.K2_GetActorLocation` _returnvalue))) (`self.detectRadius`)))
        (`BTFunctionLibrary.SetBlackboardValueAsObject` _key _returnvalue)
        (else
          (`BTFunctionLibrary.SetBlackboardValueAsObject` _key))))
    (:`Is Not Valid`
      (`BTFunctionLibrary.SetBlackboardValueAsObject` (`self.Key`)))))
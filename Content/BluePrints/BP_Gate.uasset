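; BP_Gate is a level exit gate that stays inactive, with its particles off, until ActiveGate turns it on.
; When a BP_Character enters the active gate's box, it collects the game instance's bonus money.
; After a short delay it looks up the current level in LevelInfo_DT, then has the player controller show the shop, or end the game if no next level exists.
; A separate Colaps event drops the Plane by enabling physics simulation.
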(event `self.ReceiveBeginPlay`
  (`ActorComponent.Deactivate` (`self.ParticleSystem`)))

(event `ActiveGate`
  (`ActorComponent.Activate` (`self.ParticleSystem`) false)
  (set `self.bIsActive` true))

(event `self.Box.OnComponentBeginOverlap`
  (params (OverlappedComponent :type "PrimitiveComponent Object Reference") (OtherActor :type "Actor Object Reference") (OtherComp :type "PrimitiveComponent Object Reference") (OtherBodyIndex :type Integer) (bFromSweep :type Boolean) (SweepResult :type "HitResult Structure (by ref)"))
  (if (`self.bIsActive`)
    (bind _asbp_character (cast `/Game/BluePrints/BP_CHaracter` OtherActor))
    (`/Game/BluePrints/BP_CHaracter.ColectMoney` _asbp_character (`/Game/BluePrints/BP_GameInstance.BonusMoney` (cast `/Game/BluePrints/BP_GameInstance` (`GameplayStatics.GetGameInstance`) :!pure true)))
    (`KismetSystemLibrary.Delay` 0.1)
    (bind _asbp_player_controler (cast `/Game/BluePrints/BP_PlayerControler` (`Pawn.GetController` _asbp_character)))
    (bind _returnvalue (`|GetDataTableRow` "/Game/BluePrints/LevelInfo_DT.LevelInfo_DT" (`/Game/BluePrints/BP_GameInstance.CurentLevel` (cast `/Game/BluePrints/BP_GameInstance` (`GameplayStatics.GetGameInstance`) :!pure true)))
      (:`then`
        (if (== (`.NextLevel_5_761F8AAF49F91522DC6B66AA74FB4E7C` (break `/Game/BluePrints/LevelInfo` _returnvalue)) "None")
          (`/Game/BluePrints/BP_PlayerControler.GameHasEnded` _asbp_player_controler true)
          (else
            (`/Game/BluePrints/BP_PlayerControler.ShowShop` _asbp_player_controler)))))))

(event `Colaps`
  (`PrimitiveComponent.SetSimulatePhysics` (`self.Plane`) true))

(fn `UserConstructionScript`)